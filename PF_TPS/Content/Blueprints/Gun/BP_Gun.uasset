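; Automatic hitscan rifle that manages its own ammo, HUD widget and firing effects, relying on its parent actor for aim target and reload timing.
; Fire loops at the fire rate: macros check ammo, update the reticle, play muzzle effects and line trace from the muzzle.
; Hits spawn decals, particles and sounds chosen by physical surface, and a trail moves to the impact point.
; An empty magazine triggers a delayed automatic reload.
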(event EventBeginPlay)

(event Collision|EventActorBeginOverlap
  (params (OtherActor :type Actor%20Object%20Reference)))

(event EventTick
  (params (DeltaSeconds :type Float%20%28single-precision%29)))

(event EventFire
  (params (start/stop :type Boolean))
  (bind _output_get (Variables|Fire|Setfiring start/stop))
  (if _output_get :!label _label
    (bind _p_muzzle (|PreprocessingFiring :!label _label_2))
    (bind (_out_hit_blocking_hit _out_hit_impact_point _out_hit_impact_normal _out_hit_phys_mat) (|Firing))
    (|PostprocessingFiring _out_hit_blocking_hit _out_hit_impact_point _out_hit_impact_normal _out_hit_phys_mat
      (:then
        _)
      (:false
        _))
    (Utilities|FlowControl|Sequence
      (:then_0
        (Utilities|FlowControl|Delay (Variables|Fire|Getfire_rate))
        (Components|Activation|Deactivate _p_muzzle)
        (goto _label))
      (:then_1
        (|Bullet_Trail _out_hit_impact_point)))
    (else
      (goto _label_2 false))))

(event EventEquipGun
  (Utilities|IsValid (Variables|CountAmmo|Getgun%20widget)
    (:Is%20Valid
      _)
    (:Is%20Not%20Valid
      (bind _returnvalue (UserInterface|CreateWidget (Variables|CountAmmo|Getgun%20widget%20class)))
      (Variables|CountAmmo|Setgun%20widget _returnvalue)))
  (UserInterface|Viewport|AddtoViewport (Variables|CountAmmo|Getgun%20widget) 0)
  (CallFunction|ReloadGun))

(event EventReloadGun
  (bind _magazin_capacity (Variables|CountAmmo|Getmagazin%20capacity))
  (Variables|CountAmmo|Settotal%20ammo%20count (+ (Variables|CountAmmo|Gettotal%20ammo%20count) (Variables|CountAmmo|Getloaded%20ammo%20count)))
  (Variables|CountAmmo|Setloaded%20ammo%20count (Math|Integer|SelectInt _magazin_capacity (+ (Variables|CountAmmo|Gettotal%20ammo%20count) (Variables|CountAmmo|Getloaded%20ammo%20count)) (> (- (Variables|CountAmmo|Gettotal%20ammo%20count) _magazin_capacity) 0)))
  (Variables|CountAmmo|Settotal%20ammo%20count (Math|Integer|Clamp(Integer) (- (Variables|CountAmmo|Gettotal%20ammo%20count) _magazin_capacity) 0 (Variables|CountAmmo|Getmax%20ammo%20count)))
  (CallFunction|UpdateAmmoCount))

(fn ConstructionScript)

(fn UpdateAmmoCount
  (Default|UpdateAmmoCount (Variables|CountAmmo|Getgun%20widget) (Variables|CountAmmo|Gettotal%20ammo%20count) (Variables|CountAmmo|Getloaded%20ammo%20count)))